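; BP_StarPickup is a collectible star whose mesh spins a fixed step every tick.
; Any actor overlap adds a BP_W_PickupStar widget to the viewport, and ending the overlap removes widgets of that class.
; Its PickUp event, not called within this Blueprint, increments Stars on the BP_CustomTPS reference cached at BeginPlay, clears the widget and destroys the star.
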(event EventBeginPlay
  (bind _returnvalue (Actor|GetActorOfClass "/Game/Blueprints/BP_CustomTPS.BP_CustomTPS_C"))
  (Variables|Default|SetPlayerRef _returnvalue))

(event Collision|EventActorBeginOverlap
  (params (OtherActor :type Actor%20Object%20Reference))
  (bind _returnvalue (UserInterface|CreateWidget "/Game/UI/BP_W_PickupStar.BP_W_PickupStar_C"))
  (UserInterface|Viewport|AddtoViewport _returnvalue 0))

(event EventTick
  (params (DeltaSeconds :type Float%20%28single-precision%29))
  (Transformation|AddLocalRotation (Variables|Default|GetMesh) "0,1.000000, 0" false false))

(event Collision|EventActorEndOverlap
  (params (OtherActor :type Actor%20Object%20Reference))
  (bind _foundwidgets (Widget|GetAllWidgetsOfClass "/Game/UI/BP_W_PickupStar.BP_W_PickupStar_C" true))
  (Widget|RemovefromParent _foundwidgets))

(event EventPickUp
  (bind _playerref (Variables|Default|GetPlayerRef))
  (Variables|/Game/Blueprints/BP_CustomTPS.BP_CustomTPS_C|SetStars _playerref (+ (Variables|/Game/Blueprints/BP_CustomTPS.BP_CustomTPS_C|GetStars _playerref) 1))
  (bind _foundwidgets (Widget|GetAllWidgetsOfClass "/Game/UI/BP_W_PickupStar.BP_W_PickupStar_C" true))
  (Widget|RemovefromParent _foundwidgets)
  (Actor|DestroyActor))

(fn ConstructionScript)