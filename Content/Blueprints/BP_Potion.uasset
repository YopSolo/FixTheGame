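; BP_Potion is a spinning pickup that adds one potion to the BP_CustomTPS player's count.
; Overlapping any actor shows a BP_W_Pickup widget, and ending overlap removes it via a widget class lookup.
; The PickUp event increments NumberPotions only within MaxNumberPotions, then clears the widget and destroys the potion.
; Tick rotates the mesh a fixed step per frame, unscaled by delta time.
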(event EventBeginPlay
  (bind _returnvalue (Actor|GetActorOfClass "/Game/Blueprints/BP_CustomTPS.BP_CustomTPS_C"))
  (Variables|Default|SetPlayer_ref _returnvalue))

(event Collision|EventActorBeginOverlap
  (params (OtherActor :type Actor%20Object%20Reference))
  (bind _returnvalue (UserInterface|CreateWidget "/Game/UI/BP_W_Pickup.BP_W_Pickup_C"))
  (UserInterface|Viewport|AddtoViewport _returnvalue 0))

(event EventTick
  (params (DeltaSeconds :type Float%20%28single-precision%29))
  (Transformation|AddLocalRotation (Variables|Default|GetStaticMesh) "0,1.000000, 0" false false))

(event Collision|EventActorEndOverlap
  (params (OtherActor :type Actor%20Object%20Reference))
  (bind _foundwidgets (Widget|GetAllWidgetsOfClass "/Game/UI/BP_W_Pickup.BP_W_Pickup_C" true))
  (Widget|RemovefromParent _foundwidgets))

(event EventPickUp
  (bind _player_ref (Variables|Default|GetPlayer_ref))
  (if (<= (+ (Variables|/Game/Blueprints/BP_CustomTPS.BP_CustomTPS_C|GetNumberPotions _player_ref) 1) (Variables|/Game/Blueprints/BP_CustomTPS.BP_CustomTPS_C|GetMaxNumberPotions _player_ref))
    (Variables|/Game/Blueprints/BP_CustomTPS.BP_CustomTPS_C|SetNumberPotions _player_ref (+ (Variables|/Game/Blueprints/BP_CustomTPS.BP_CustomTPS_C|GetNumberPotions _player_ref) 1))
    (bind _foundwidgets (Widget|GetAllWidgetsOfClass "/Game/UI/BP_W_Pickup.BP_W_Pickup_C" true))
    (Widget|RemovefromParent _foundwidgets)
    (Actor|DestroyActor)))

(fn ConstructionScript)