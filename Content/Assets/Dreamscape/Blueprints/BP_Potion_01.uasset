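; BP_Potion_01 is a collectible health potion pickup for the BP_CustomTPS player character.
; On any actor overlap it casts player 0's character, increments its PotionScore, adds a fixed heal to CurrentHealth clamped to MaxHealth, then destroys itself.
; It never checks the overlapping actor, so any overlap credits the player.
; An empty mesh overlap event and an unconnected older heal chain with a hardcoded cap remain unused.
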(event OnComponentBeginOverlap(StaticMesh)
  (params (OverlappedComponent :type Primitive%20Component%20Object%20Reference) (OtherActor :type Actor%20Object%20Reference) (OtherComp :type Primitive%20Component%20Object%20Reference) (OtherBodyIndex :type Integer) (bFromSweep :type Boolean) (SweepResult :type Hit%20Result%20Structure%20%28by%20ref%29)))

(event Collision|EventActorBeginOverlap
  (params (OtherActor :type Actor%20Object%20Reference))
  (bind _asbp_custom_tps (Utilities|Casting|CastToBP_CustomTPS (Game|GetPlayerCharacter 0)))
  (Variables|/Game/Blueprints/BP_CustomTPS.BP_CustomTPS_C|SetPotionScore _asbp_custom_tps (+ (Variables|/Game/Blueprints/BP_CustomTPS.BP_CustomTPS_C|GetPotionScore _asbp_custom_tps) 1))
  (Variables|/Game/Blueprints/BP_CustomTPS.BP_CustomTPS_C|SetCurrentHealth _asbp_custom_tps (Math|Float|Clamp(Float) (+ (Variables|/Game/Blueprints/BP_CustomTPS.BP_CustomTPS_C|GetCurrentHealth _asbp_custom_tps) 1e+01) 0.0 (Variables|/Game/Blueprints/BP_CustomTPS.BP_CustomTPS_C|GetMaxHealth _asbp_custom_tps)))
  (Actor|DestroyActor))

(fn ConstructionScript)